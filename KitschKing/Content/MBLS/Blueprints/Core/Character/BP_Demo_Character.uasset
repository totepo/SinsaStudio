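; Demo player character that applies the player's saved appearance, a body skeletal mesh and a hat, and replicates it.
; An owning-client init event reads both meshes from the local appearance save and passes them to server update events, skipping failed loads.
; The server events set the current mesh variables, whose OnRep functions apply them to the character mesh (when valid) and the hat slot's static mesh component.
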(event Custom|SR_Update_SkeletalMesh
  (params (SkeletalMesh :type Skeletal%20Mesh%20Object%20Reference))
  ;[0.05448 0.05448 0.05448] Appearance Updates
  (Variables|Appearance|SetCurrent_SkeletalMesh SkeletalMesh))

(event Custom|SR_Update_Hat
  (params (Hat :type Static%20Mesh%20Object%20Reference))
  ;[0.05448 0.05448 0.05448] Appearance Updates
  (Variables|Appearance|SetCurrent_HatSlot Hat))

(event Custom|OC_Init_Appearance
  ;[0.05098 0.05098 0.05098] Initialize player appearance
  (Player|Appearance|GetPlayerAppearance))

(fn ConstructionScript)

(fn OnRepCurrentSkeletalMesh
  (bind _current_skeletalmesh (Variables|Appearance|GetCurrent_SkeletalMesh)
    (:then
      (Components|SkinnedMesh|SetSkinnedAssetandUpdate (Variables|Character|GetMesh) _current_skeletalmesh false))
    (:else)))

(fn OnRepCurrentHatSlot
  (Components|StaticMesh|SetStaticMesh (Variables|Default|GetHat_Slot) (Variables|Appearance|GetCurrent_HatSlot)))

(fn GetPlayerAppearance
  ;[0.05098 0.05098 0.05098] Load the player appearance from the local player appearance save file, and update the character with it
  (Player|Appearance|GetSkeletalMesh)
  (Player|Appearance|GetHat))

(fn GetSkeletalMesh
  ;[0.05098 0.05098 0.05098] Get the player's Character from the save game and update the server
  (bind (_s_playerappearance _succes_) (CallFunction|GetPlayerAppearance))
  (if _succes_
    (CallFunction|SRUpdateSkeletalMesh (.Mesh (Utilities|Struct|BreakS_Available_Characters (.Character (Utilities|Struct|BreakS_Player_Appearance _s_playerappearance)))))
    (return)
    (else
      (return))))

(fn GetHat
  ;[0.05098 0.05098 0.05098] Get the player's Hat Slot item from the save game and update the server
  (bind (_s_playerappearance _succes_) (CallFunction|GetPlayerAppearance))
  (if _succes_
    (CallFunction|SRUpdateHat (.Mesh (Utilities|Struct|BreakS_Available_Accessories_Hat (.Hat_Slot (Utilities|Struct|BreakS_Player_Appearance _s_playerappearance)))))
    (return)
    (else
      (return))))