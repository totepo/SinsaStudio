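; Death zone for the City stage: a cube that shifts vertically in three timed stages during a match.
; Tick compares the game state's IngameTime with three trigger times, each driving a timeline that sets the cube's relative Z and flags its stage done on finish.
; Once the game has started, overlaps on the server notify the other actor through an interface death-zone message.
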(event OnComponentBeginOverlap(Cube)
  (params (OverlappedComponent :type Primitive%20Component%20Object%20Reference) (OtherActor :type Actor%20Object%20Reference) (OtherComp :type Primitive%20Component%20Object%20Reference) (OtherBodyIndex :type Integer) (bFromSweep :type Boolean) (SweepResult :type Hit%20Result%20Structure%20%28by%20ref%29))
  (Networking|SwitchHasAuthority
    (:Authority
      (if (Variables|/Game/ThirdPerson/Blueprints/MainGame/GS_MainGame.GS_MainGame_C|GetGame%20Start (Variables|Default|GetAs%20GS%20Main%20Game))
        (Utilities|IsValid OtherActor
          (:Is%20Valid
            (Class|BPIDeathzone|InterfaceonDeathZone(Message) OtherActor)))))))

(event Custom|Event%20Trigger%202
  (bind _cube (Variables|Default|GetCube))
  (bind _relativelocation (Variables|/Script/Engine.SceneComponent|GetRelativeLocation _cube))
  (bind _z_location (Timeline|Timeline_1 Play)
    (:Update
      (bind _output_get (Variables|Default|SetRelative%20Location (Math|Vector|MakeVector (.x _relativelocation) (.y _relativelocation) (/ _z_location 5.0))))
      (Transformation|SetRelativeLocation (Variables|Default|GetCube) _output_get false false))
    (:Finished
      (Variables|Default|SetTrigger_2_Done true))))

(event Custom|Event%20Trigger%203
  (bind _cube (Variables|Default|GetCube))
  (bind _relativelocation (Variables|/Script/Engine.SceneComponent|GetRelativeLocation _cube))
  (bind _newtrack_0 (Timeline|Timeline_2 Play)
    (:Update
      (bind _output_get (Variables|Default|SetRelative%20Location (Math|Vector|MakeVector (.x _relativelocation) (.y _relativelocation) (/ _newtrack_0 5.0))))
      (Transformation|SetRelativeLocation (Variables|Default|GetCube) _output_get false false))
    (:Finished
      (Variables|Default|SetTrigger_3_Done true))))

(event Custom|Event%20Trigger%201
  (bind _cube (Variables|Default|GetCube))
  (bind _relativelocation (Variables|/Script/Engine.SceneComponent|GetRelativeLocation _cube))
  (bind _z_relative_location (Timeline|Timeline Play)
    (:Update
      (bind _output_get (Variables|Default|SetRelative%20Location (Math|Vector|MakeVector (.x _relativelocation) (.y _relativelocation) (/ _z_relative_location 5.0))))
      (Transformation|SetRelativeLocation (Variables|Default|GetCube) _output_get false false))
    (:Finished
      (Variables|Default|SetTrigger_1_Done true))))

(event EventBeginPlay
  (bind _asgs_main_game (Utilities|Casting|CastToGS_MainGame (Game|GetGameState)))
  (Variables|Default|SetAs%20GS%20Main%20Game _asgs_main_game))

(event EventTick
  (params (DeltaSeconds :type Float%20%28single-precision%29))
  (Utilities|FlowControl|Sequence
    (:then_0
      (if (and (> (Variables|/Game/ThirdPerson/Blueprints/MainGame/GS_MainGame.GS_MainGame_C|GetIngame_Time (Variables|Default|GetAs%20GS%20Main%20Game)) (Variables|Default|GetTriggerTime_1)) (not (Variables|Default|GetTrigger_1_Done)))
        (CallFunction|EventTrigger1)))
    (:then_1
      (if (and (> (Variables|/Game/ThirdPerson/Blueprints/MainGame/GS_MainGame.GS_MainGame_C|GetIngame_Time (Variables|Default|GetAs%20GS%20Main%20Game)) (Variables|Default|GetTriggerTime_2)) (not (Variables|Default|GetTrigger_2_Done)))
        (CallFunction|EventTrigger2)))
    (:then_2
      (if (and (> (Variables|/Game/ThirdPerson/Blueprints/MainGame/GS_MainGame.GS_MainGame_C|GetIngame_Time (Variables|Default|GetAs%20GS%20Main%20Game)) (Variables|Default|GetTriggerTime_3)) (not (Variables|Default|GetTrigger_3_Done)))
        (CallFunction|EventTrigger3)))))

(fn ConstructionScript)